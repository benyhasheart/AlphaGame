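; BP_Canvas is a paintable canvas actor that accumulates brush strokes in a render target.
; BeginPlay creates a white-cleared render target, shows it on the Canvas component through an M_Canvas dynamic material, and creates an M_Brush dynamic material.
; DrawBrush sets the brush texture, then draws that material into the render target at a given size, centered on a normalized draw location.
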(event `self.ReceiveBeginPlay`
  (`|ExecutionSequence`
    (:`then_0`
      (bind _returnvalue (`KismetRenderingLibrary.CreateRenderTarget2D` 256))
      (bind _output_get (set `self.Rendertarget` _returnvalue))
      (`KismetRenderingLibrary.ClearRenderTarget2D` _output_get (struct :`R` 1.0 :`G` 1.0 :`B` 1.0 :`A` 1.0)))
    (:`then_1`
      (bind _returnvalue_2 (`KismetMaterialLibrary.CreateDynamicMaterialInstance` "/Game/PaintMesh/Materials/M_Canvas.M_Canvas"))
      (`MaterialInstanceDynamic.SetTextureParameterValue` _returnvalue_2 "Rendertarget" (`self.Rendertarget`))
      (`PrimitiveComponent.SetMaterial` (`self.Canvas`) 0 _returnvalue_2))
    (:`then_2`
      (bind _returnvalue_3 (`KismetMaterialLibrary.CreateDynamicMaterialInstance` "/Game/PaintMesh/Materials/M_Brush.M_Brush"))
      (set `self.Brushmaterial` _returnvalue_3))))

(fn `DrawBrush`
  (params (Brushtexture :type "Texture2D Object Reference") (BrushSize :type "Float (double-precision)") (DrawLocation :type "Vector2D Structure"))
  (bind _brushsize (`local.BrushSize`))
  (`|ExecutionSequence`
    (:`then_0`
      (`MaterialInstanceDynamic.SetTextureParameterValue` (`self.Brushmaterial`) "BrushTexture" Brushtexture))
    (:`then_1`
      (bind (_canvas _size _context) (`KismetRenderingLibrary.BeginDrawCanvasToRenderTarget` (`self.Rendertarget`)))
      (`Canvas.K2_DrawMaterial` _canvas (`self.Brushmaterial`) (- (* _size (`local.DrawLocation`)) (/ _brushsize 2.0)) (`KismetMathLibrary.MakeVector2D` _brushsize _brushsize) (0.0 0.0) (1.0 1.0) 0.0 (0.5 0.5))
      (`KismetRenderingLibrary.EndDrawCanvasToRenderTarget` _context))))

(fn `UserConstructionScript`)