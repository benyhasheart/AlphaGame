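; BP_Pawn is a player pawn that paints on BP_Canvas actors in the level.
; BeginPlay adds the IMC_Play Enhanced Input mapping context for its player controller.
; While IA_Paint triggers, it runs a complex Visibility line trace forward from the camera.
; On a canvas hit, it converts the hit to a UV with FindCollisionUV and passes it, with brush texture and size, to DrawBrush.
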(event `self.ReceiveBeginPlay`
  (bind _asplayer_controller (cast `PlayerController` (`self.GetController`)))
  (bind _returnvalue (pcsubsystem `EnhancedInputLocalPlayerSubsystem` _asplayer_controller))
  (`/Engine/EditorBlueprintResources/StandardMacros.IsValid` _returnvalue
    (:`Is Valid`
      (`EnhancedInputSubsystemInterface.AddMappingContext` _returnvalue "/Game/PaintMesh/Blueprints/IMC_Play.IMC_Play" 0 (struct)))))

(event `EnhancedInput|/Game/PaintMesh/Blueprints/IA_Paint`
  (params (ActionValue :type "Float (double-precision)") (ElapsedSeconds :type "Float (double-precision)") (TriggeredSeconds :type "Float (double-precision)") (InputAction :type "InputAction Object Reference" :default "/Game/PaintMesh/Blueprints/IA_Paint.IA_Paint"))
  (bind _returnvalue (`GameplayStatics.GetPlayerCameraManager` 0))
  (bind _returnvalue_2 (`self.K2_GetActorLocation` _returnvalue))
  (:`Triggered`
    (if (== ActionValue 1.0)
      (bind _outhit (`KismetSystemLibrary.LineTraceSingle` _returnvalue_2 (+ _returnvalue_2 (* (`self.GetActorForwardVector` _returnvalue) 1000.0)) "TraceTypeQuery1" true))
      (bind _asbp_canvas (cast `/Game/PaintMesh/Blueprints/BP_Canvas` (`.HitActor` (`GameplayStatics.BreakHitResult` _outhit))))
      (`/Game/PaintMesh/Blueprints/BP_Canvas.DrawBrush` _asbp_canvas (`self.Brushtexture`) (`self.Brush Size`) (`GameplayStatics.FindCollisionUV` _outhit)))))

(fn `UserConstructionScript`)